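; BP_PlayerController is the player controller that turns Enhanced Input actions into movement, look and firing on the possessed character.
; BeginPlay casts the controlled pawn to CharacterBase, caches it, and adds the default input mapping context only if that cast succeeds.
; Look drives controller yaw and pitch, while move, jump and fire start/stop are forwarded to the cached character.
; Weapon swap and utility actions are empty stubs.
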(event Input|EnhancedActionEvents|EnhancedInputActionIA_Move
  (params (ActionValue :type Vector%202D%20Structure) (ElapsedSeconds :type Float%20%28double-precision%29) (TriggeredSeconds :type Float%20%28double-precision%29) (InputAction :type Input%20Action%20Object%20Reference :default "/Game/Input/Actions/IA_Move.IA_Move"))
  (bind _controlledcharacter (Variables|Default|GetControlledCharacter))
  ;[1 1 1] Movement
  (:Triggered
    (Pawn|Input|AddMovementInput _controlledcharacter (Transformation|GetActorRightVector _controlledcharacter) (.x ActionValue) false)
    (Pawn|Input|AddMovementInput _controlledcharacter (Transformation|GetActorForwardVector _controlledcharacter) (.y ActionValue) false)))

(event Input|EnhancedActionEvents|EnhancedInputActionIA_Look
  (params (ActionValue :type Vector%202D%20Structure) (ElapsedSeconds :type Float%20%28double-precision%29) (TriggeredSeconds :type Float%20%28double-precision%29) (InputAction :type Input%20Action%20Object%20Reference :default "/Game/Input/Actions/IA_Look.IA_Look"))
  (bind (_x _y) (Math|Vector2D|BreakVector2D ActionValue))
  ;[1 1 1] Movement
  (Class|PlayerController|AddYawInput _x)
  (Class|PlayerController|AddPitchInput _y))

(event Input|EnhancedActionEvents|EnhancedInputActionIA_SwapWeapon
  (params (ActionValue :type Boolean) (ElapsedSeconds :type Float%20%28double-precision%29) (TriggeredSeconds :type Float%20%28double-precision%29) (InputAction :type Input%20Action%20Object%20Reference :default "/Game/Input/Actions/IA_SwapWeapon.IA_SwapWeapon")))

(event Input|EnhancedActionEvents|EnhancedInputActionIA_UtilityAction
  (params (ActionValue :type Boolean) (ElapsedSeconds :type Float%20%28double-precision%29) (TriggeredSeconds :type Float%20%28double-precision%29) (InputAction :type Input%20Action%20Object%20Reference :default "/Game/Input/Actions/IA_UtilityAction.IA_UtilityAction")))

(event Input|EnhancedActionEvents|EnhancedInputActionIA_FireWeapon
  (params (ActionValue :type Boolean) (ElapsedSeconds :type Float%20%28double-precision%29) (TriggeredSeconds :type Float%20%28double-precision%29) (InputAction :type Input%20Action%20Object%20Reference :default "/Game/Input/Actions/IA_FireWeapon.IA_FireWeapon"))
  (bind _controlledcharacter (Variables|Default|GetControlledCharacter))
  (:Started
    (Class|CharacterBase|StartFire _controlledcharacter))
  (:Completed
    (Class|CharacterBase|StopFire _controlledcharacter)))

(event Input|EnhancedActionEvents|EnhancedInputActionIA_Jump
  (params (ActionValue :type Boolean) (ElapsedSeconds :type Float%20%28double-precision%29) (TriggeredSeconds :type Float%20%28double-precision%29) (InputAction :type Input%20Action%20Object%20Reference :default "/Game/Input/Actions/IA_Jump.IA_Jump"))
  (:Ongoing
    (Character|Jump (Variables|Default|GetControlledCharacter))))

(event EventBeginPlay
  (bind _ascharacter_base (Utilities|Casting|CastToCharacterBase (Pawn|GetControlledPawn)))
  (Variables|Default|SetControlledCharacter _ascharacter_base)
  (Input|AddMappingContext (PlayerController|LocalPlayerSubsystems|GetEnhancedInputLocalPlayerSubsystem) "/Game/Input/IMC_Default.IMC_Default" 0 "(bIgnoreAllPressedKeysUntilRelease=True,bForceImmediately=False,bNotifyUserSettings=False)"))

(fn ConstructionScript)