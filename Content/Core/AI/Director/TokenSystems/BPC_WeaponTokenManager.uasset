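; Director component that rations weapon tokens among controlled AI, scaled by difficulty.
; It binds to each AI's weapon-fired event and keeps a shared shot count against a threshold from a per-difficulty curve, sampled using eligible AI and perceived actor counts.
; At the threshold, it resets the count and grants a token to a random AI's weapon, choosing among tokenless AI that perceive any of the tracked sighted actors.
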(event Custom|OnDifficultyChanged_Event
  (params (Difficulty :type Integer))
  (Variables|Default|SetDifficulty Difficulty))

(event Custom|OnUpdatedSight
  (params (PercievedActors :type Array%20of%20Actor%20Object%20References))
  (Variables|Default|SetPercievedActors PercievedActors))

(event Custom|OnWeaponFired
  (params (Weapon :type Weapon%20Base%20Object%20Reference) (OwnedCharacter :type Character%20Base%20Object%20Reference))
  (bind _assignable (CallFunction|GetActorsPercieving))
  (Variables|Default|SetTokenShotCount (Math|Float|Round (Class|KismetMathLibrary|GetRuntimeFloatCurveValue (Utilities|Array|Get(acopy) (Variables|Default|GetPercivingTokenReduction) (Variables|Default|GetDifficulty)) (Math|Conversions|ToFloat(Integer) (- (+ (Utilities|Array|Length _assignable) 2) (Utilities|Array|Length (Variables|Default|GetPercievedActors)))) 1.0)))
  (bind _result (Math|Integer|IncrementInt (Variables|Default|GetCurrentShots))
    (:%20%20
      (if (>= _result (Variables|Default|GetTokenShotCount))
        (Development|PrintString "Add Token" false)
        (Variables|Default|SetCurrentShots 0)
        (bind _assignable_2 (CallFunction|GetActorsPercieving))
        (if (!= (Utilities|Array|Length _assignable_2) 0)
          (bind _asbp_aicharacter (Utilities|Casting|CastToBP_AICharacter (Pawn|GetControlledPawn (Utilities|Array|Get(acopy) _assignable_2 (Math|Random|RandomIntegerinRange 0 (- (Utilities|Array|Length _assignable_2) 1))))))
          (bind _returnvalue (Class|CharacterBase|GetCurrentWeapon _asbp_aicharacter))
          (Class|WeaponBase|SetTokenState _returnvalue true))
        (else
          (Development|PrintString "Not Enough Shots Fired" false false "(R=1.000000,G=0.000000,B=0.191897,A=1.000000)"))))))

(event Custom|InitTokenManager
  (params (Controlled%20AI :type Array%20of%20AI%20Controller%20Base%20Object%20References))
  (bind _output_get (Variables|Default|SetControlled%20AI Controlled%20AI))
  (for _array_element _output_get
    (EventDispatchers|BindEventtoOnAICWeaponFired _array_element (EventDispatchers|CreateEvent :!event Custom|OnWeaponFired))))

(event EventBeginPlay
  (bind _asbp_director_base (Utilities|Casting|CastToBP_DirectorBase (Components|GetOwner)))
  (EventDispatchers|AssignOnDifficultyChanged _asbp_director_base (delegate Custom|OnDifficultyChanged_Event)))

(fn GetActorsPercieving
  (bind _tokenassignable (LocalVariables|GetTokenAssignable))
  (Utilities|Array|Clear (LocalVariables|GetTokenAssignable))
  (for _array_element (Variables|Default|GetControlled%20AI)
    (bind _returnvalue (Class|AIControllerBase|GetPercievedActors _array_element))
    (bind _output_get (LocalVariables|SetTempPercieved _returnvalue))
    (for _array_element_2 (Variables|Default|GetPercievedActors)
      (if (Utilities|Array|ContainsItem _output_get _array_element_2)
        (bind _asbp_aicharacter (Utilities|Casting|CastToBP_AICharacter (Pawn|GetControlledPawn _array_element)))
        (bind _returnvalue_2 (Class|CharacterBase|GetCurrentWeapon _asbp_aicharacter))
        (if (not (Variables|/Script/Director_System.WeaponBase|GetbHasToken _returnvalue_2))
          (if (not (Utilities|Array|ContainsItem _tokenassignable _array_element))
            (Utilities|Array|AddUnique _tokenassignable _array_element))))))
  (return (LocalVariables|GetTokenAssignable)))