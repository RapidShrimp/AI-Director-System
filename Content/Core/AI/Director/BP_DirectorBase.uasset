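; BP_DirectorBase is a base AI director that tracks which enemies its controlled AI can see as a group.
; It listens to its spawn controller, registers each spawned AI and binds to that agent's sight updates.
; Sighted enemies join a shared list and leave it when sight is lost and no controlled AI still perceives them.
; The enemy spotted and lost functions are empty stubs.
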(event Custom|OnAISpawned
  (params (SpawnedAI :type AI%20Sensing%20Controller%20Object%20Reference))
  (EventDispatchers|BindEventtoOnEnemySightUpdated SpawnedAI (EventDispatchers|CreateEvent :!event OnAgentSightUpdated))
  (Utilities|Array|AddUnique (Variables|Default|GetControlled%20AI) SpawnedAI))

(event EventBeginPlay
  (bind _controlspawn (Variables|Default|GetControlSpawn)
    (:then
      (EventDispatchers|BindEventtoOnAISpawned _controlspawn (EventDispatchers|CreateEvent :!event Custom|OnAISpawned)))
    (:else)))

(fn ConstructionScript)

(fn OnAgentSightUpdated
  (params (AISpotting :type AI%20Sensing%20Controller%20Object%20Reference) (SpottedEnemy :type Actor%20Object%20Reference) (HasSight :type Boolean))
  (if HasSight
    (if (not (Utilities|Array|ContainsItem (Variables|Default|GetSightedEnemies) SpottedEnemy))
      (Utilities|Array|AddUnique (Variables|Default|GetSightedEnemies) SpottedEnemy))
    (else
      (bind _percievedactors (CallFunction|GetAIPercievedActors))
      (if (not (Utilities|Array|ContainsItem _percievedactors SpottedEnemy))
        (Utilities|Array|RemoveItem (Variables|Default|GetSightedEnemies) SpottedEnemy)))))

(fn GetAIPercievedActors
  (for _array_element (Variables|Default|GetControlled%20AI)
    (bind _percievedactors (Default|GetPercievedActors _array_element))
    (for _array_element_2 _percievedactors
      (if (not (Utilities|Array|ContainsItem (LocalVariables|GetPercievedTotal) _array_element_2))
        (Utilities|Array|AddUnique (LocalVariables|GetPercievedTotal) _array_element_2))))
  (return (LocalVariables|GetPercievedTotal)))

(fn OnEnemySpotted
  (params (SpottedEnemy :type Actor%20Object%20Reference)))

(fn OnEnemyLost
  (params (EnemyLostSight :type Actor%20Object%20Reference)))